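; AC_Combat is an actor component that manages its owner's weapons: spawning, switching, firing and reloading.
; BuildWeapons spawns each configured class, attaches it to a socket on the supplied hands component, optionally fills its ammo and shows only the first.
; ChangeWeapon uses the weapon type enum as the map key to swap visibility and the equipped reference, notifying through OnChangeWeapon.
; Firing, shoot checks, reloading and attribute queries pass through to the equipped weapon.
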(event `Fire Equipped Weapon`
  (params (`Foward Vector` :type "Vector Structure") (`Player Is Aiming` :type Boolean))
  (`/Game/Blueprints/Actors/BP_BaseWeapon.Fire` (`self.Equipped Weapon`) `Foward Vector` `Player Is Aiming`))

(fn `Build Weapons`
  (params (`Player Hands` :type "SkeletalMeshComponent Object Reference"))
  (locals (Key :type Integer))
  (bind (_value _returnvalue) (`BlueprintMapLibrary.Map_Find` (`self.Weapons Map`)))
  (for (_array_element _array_index) (`self.Weapon Classes`)
    (set `local.Key` _array_index)
    (bind _returnvalue_2 (`|SpawnActorFromClass` _array_element (`Actor.GetTransform` (`self.GetOwner`)) "AlwaysSpawn" "MultiplyWithRoot" (`self.GetOwner`) null))
    (`BlueprintMapLibrary.Map_Add` (`self.Weapons Map`) (`local.Key`) _returnvalue_2)
    (`Actor.K2_AttachToComponent` _returnvalue_2 (`local.Player Hands`) (`self.Weapon Socket Name`) "SnapToTarget" "SnapToTarget" "SnapToTarget" false)
    (if (`self.Add Ammo To All Weapon`)
      (bind _weapon_attributes (`/Game/Blueprints/Actors/BP_BaseWeapon.Weapon Attributes` _returnvalue_2))
      (set `/Game/Blueprints/Data/PDA_Weapon.Current Ammo Count` (`/Game/Blueprints/Data/PDA_Weapon.Max Ammo Count` _weapon_attributes) _weapon_attributes)
      (set `/Game/Blueprints/Data/PDA_Weapon.Current Clip Amount` (`/Game/Blueprints/Data/PDA_Weapon.Clip Size` _weapon_attributes) _weapon_attributes)))
  (bind _values (`BlueprintMapLibrary.Map_Values` (`self.Weapons Map`)))
  (for _array_element_2 _values
    (`Actor.SetActorHiddenInGame` _array_element_2 true))
  (if _returnvalue
    (`Actor.SetActorHiddenInGame` _value false)
    (set `self.Equipped Weapon` _value)
    (set `self.Current Weapon Type` "NewEnumerator0")))

(fn `Can Shoot Weapon`
  (returns (`Can Shoot Again` :type Boolean))
  (return (`/Game/Blueprints/Actors/BP_BaseWeapon.Can Shoot` (`self.Equipped Weapon`))))

(fn `Change Weapon`
  (params (`Weapon Type` :type "/Game/Blueprints/Enums/E_PlayerWeapons Enum" :default "NewEnumerator0"))
  (bind (_value _returnvalue) (`BlueprintMapLibrary.Map_Find` (`self.Weapons Map`) (`KismetMathLibrary.Conv_ByteToInt` (`self.Current Weapon Type`))))
  (bind _output_get (set `self.Current Weapon Type` `Weapon Type`))
  (`self.OnChangeWeapon` _output_get)
  (`Actor.SetActorHiddenInGame` (`self.Equipped Weapon`) true)
  (if _returnvalue
    (bind _output_get_2 (set `self.Equipped Weapon` _value))
    (`Actor.SetActorHiddenInGame` _output_get_2 false)))

(fn `Get Equipped Weapon Attributes`
  (returns (`Weapon Attributes` :type "/Game/Blueprints/Data/PDA_Weapon Object Reference"))
  (return (`/Game/Blueprints/Actors/BP_BaseWeapon.Weapon Attributes` (`self.Equipped Weapon`))))

(fn `Reload Equipped Weapon`
  (`/Game/Blueprints/Actors/BP_BaseWeapon.Reload Weapon` (`self.Equipped Weapon`)))