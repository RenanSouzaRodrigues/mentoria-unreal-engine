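; Shotgun weapon actor that fires multiple spread hitscan traces and gates refiring on its fire animation.
; Each shot randomizes trace endpoints through WeaponAttributes spread, deals damage via BPI_Damageable and spawns damage numbers with critical-hit info.
; The fire montage runs alongside a camera shake, and its completion clears the shell-loading flag to allow the next shot.
; Traces use the Visibility channel and draw debug lines.
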(event `self.Fire`
  (params (`Foward Vector` :type "Vector Structure"))
  (bind _returnvalue (`SceneComponent.K2_GetComponentLocation` (`self.Arrow`)))
  (if (`self.Can Shoot Again`)
    (set `self.Can Shoot Again` false)
    (`self.Perform Fire Trace` _returnvalue (+ _returnvalue (* `Foward Vector` (`/Game/Blueprints/Data/PDA_Weapon.Weapon Range` (`self.Weapon Attributes`)))))
    (`|PlayMontage` (`self.Weapon Body`) (`self.Fire Montage`)
      (:`then`
        (set `self.Is Loading Next Shell` true)
        (`PlayerCameraManager.StartCameraShake` :`self` (`GameplayStatics.GetPlayerCameraManager` 0) :`ShakeClass` (`self.Fire Camera Shake`)))
      (:`OnCompleted`
        (set `self.Is Loading Next Shell` false)
        (`self.Reset`)))))

(event `self.Reset`
  (if (not (`self.Is Loading Next Shell`))
    (set `self.Can Shoot Again` true)))

(fn `Perform Fire Trace`
  (params (Start :type "Vector Structure") (End :type "Vector Structure"))
  (for _ (range (+ (`self.Amount Of Traces`) 1))
    (bind _outhit (`KismetSystemLibrary.LineTraceSingle` :`Start` (`local.Start`) :`End` (+ (`local.End`) (`KismetMathLibrary.MakeVector` 0.0 (`/Game/Blueprints/Data/PDA_Weapon.Calculate Spread` (`self.Weapon Attributes`)) (`/Game/Blueprints/Data/PDA_Weapon.Calculate Spread` (`self.Weapon Attributes`)))) :`TraceChannel` "TraceTypeQuery1" :`DrawDebugType` "ForDuration"))
    (bind (_bblockinghit _binitialoverlap _time _distance _location _impactpoint _normal _impactnormal _physmat _hitactor) (`GameplayStatics.BreakHitResult` _outhit))
    (if (`KismetSystemLibrary.DoesImplementInterface` _hitactor "/Game/Blueprints/Interfaces/BPI_Damageable.BPI_Damageable_C")
      (bind (_damage_received _critical_hit) (message `/Game/Blueprints/Interfaces/BPI_Damageable.Deal Damage` _hitactor (`/Game/Blueprints/Data/PDA_Weapon.Calculate Damage` (`self.Weapon Attributes`))))
      (`/Game/Blueprints/Components/AC_DamageNumbers.Spawn Damage Numbers` (`self.Damage Numbers`) (`KismetMathLibrary.FTrunc` _damage_received) _critical_hit _hitactor _impactpoint)))
  (return))

(fn `UserConstructionScript`
  (`parent.UserConstructionScript`))