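; First-person player character that handles movement, look, aim, sprint, shooting, reloading and switching between four weapons through Enhanced Input.
; A player state sets walk speed, while a timeline zooms camera FOV for aiming and input checks arbitrate aim against sprint.
; CombatComponent runs weapon logic and reports changes to the HUD; PlayerInventory gates non-pistol weapons.
; Arm montages are looked up by weapon and aim state, with reload applied on montage completion.
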(event `self.ReceiveBeginPlay`
  (`self.Set New Player State` "NewEnumerator0")
  (add `/Game/Blueprints/Components/AC_Combat.OnChangeWeapon` (`self.Combat Component`) (`|CreateDelegate` :!event `On Change Weapon Event Listener`))
  (`/Game/Blueprints/Components/AC_Combat.Build Weapons` (`self.Combat Component`) (`self.Player Arms`))
  (bind _returnvalue (`|CreateWidget` "/Game/Blueprints/Huds/WBP_PlayerUI.WBP_PlayerUI_C"))
  (bind _output_get (set `self.Player UI` _returnvalue))
  (`UserWidget.AddToViewport` _output_get 0))

(event `On Change Weapon Event Listener`
  (params (`Weapon Type` :type "/Game/Blueprints/Enums/E_PlayerWeapons Enum" :default "NewEnumerator0"))
  (set `self.Is Changing Weapon` true)
  (set `self.Current Weapon` `Weapon Type`)
  (`/Game/Blueprints/Huds/WBP_PlayerUI.Change Crosshair` (`self.Player UI`) (`self.Current Weapon`))
  (`/Game/Blueprints/Huds/WBP_PlayerUI.Change Image` (`self.Player UI`) (`self.Current Weapon`))
  (`/Game/Blueprints/Huds/WBP_PlayerUI.Update Equipped Weapon` (`self.Player UI`) (`/Game/Blueprints/Components/AC_Combat.Get Equipped Weapon Attributes` (`self.Combat Component`))))

(event `EnhancedInput|/Game/Blueprints/Inputs/IA_Movement`
  (params (ActionValue :type "Vector2D Structure") (ElapsedSeconds :type "Float (double-precision)") (TriggeredSeconds :type "Float (double-precision)") (InputAction :type "InputAction Object Reference" :default "/Game/Blueprints/Inputs/IA_Movement.IA_Movement"))
  (bind (_x _y) (`KismetMathLibrary.BreakVector2D` ActionValue))
  ;[0 1 0.2865] Movement
  (:`Triggered`
    (`self.AddMovementInput` (`self.GetActorForwardVector`) _x)
    (`self.AddMovementInput` (`self.GetActorRightVector`) _y)))

(event `EnhancedInput|/Game/Blueprints/Inputs/IA_Look`
  (params (ActionValue :type "Vector2D Structure") (ElapsedSeconds :type "Float (double-precision)") (TriggeredSeconds :type "Float (double-precision)") (InputAction :type "InputAction Object Reference" :default "/Game/Blueprints/Inputs/IA_Look.IA_Look"))
  (bind (_x _y) (`KismetMathLibrary.BreakVector2D` ActionValue))
  ;[0 1 0.2865] Look
  (:`Triggered`
    (`self.AddControllerYawInput` _x)
    (`self.AddControllerPitchInput` _y)))

(event `EnhancedInput|/Game/Blueprints/Inputs/IA_Aim`
  (params (ActionValue :type Boolean) (ElapsedSeconds :type "Float (double-precision)") (TriggeredSeconds :type "Float (double-precision)") (InputAction :type "InputAction Object Reference" :default "/Game/Blueprints/Inputs/IA_Aim.IA_Aim"))
  ;[0 1 0.2865] Aim
  (:`Started`
    (`self.Set New Player State` "NewEnumerator1")
    (bind (_direction _field_of_view) (`Timeline|Aim Zoom Timeline` :!label _label)
      (:`Update`
        (`CameraComponent.SetFieldOfView` (`self.Camera`) _field_of_view))))
  (:`Canceled`
    (if (`|GetInputActionValue`) :!label _label_2
      (`self.Set New Player State` "NewEnumerator3")
      (goto _label :!via `Reverse`)
      (else
        (`self.Set New Player State` "NewEnumerator0")
        (goto _label :!via `Reverse`))))
  (:`Completed`
    (goto _label_2)))

(event `EnhancedInput|/Game/Blueprints/Inputs/IA_Sprint`
  (params (ActionValue :type Boolean) (ElapsedSeconds :type "Float (double-precision)") (TriggeredSeconds :type "Float (double-precision)") (InputAction :type "InputAction Object Reference" :default "/Game/Blueprints/Inputs/IA_Sprint.IA_Sprint"))
  ;[0 1 0.2865] Sprint
  (:`Started`
    (`self.Set New Player State` "NewEnumerator3")
    (if (`|GetInputActionValue`)
      (`TimelineComponent.Reverse` (`self.Aim Zoom Timeline`))))
  (:`Canceled`
    (if (`|GetInputActionValue`) :!label _label_3
      (if (not (`self.Is Aiming`))
        (`self.Set New Player State` "NewEnumerator1")
        (`TimelineComponent.PlayFromStart` (`self.Aim Zoom Timeline`)))
      (else
        (`self.Set New Player State` "NewEnumerator0"))))
  (:`Completed`
    (goto _label_3)))

(event `EnhancedInput|/Game/Blueprints/Inputs/IA_Shoot`
  (params (ActionValue :type Boolean) (ElapsedSeconds :type "Float (double-precision)") (TriggeredSeconds :type "Float (double-precision)") (InputAction :type "InputAction Object Reference" :default "/Game/Blueprints/Inputs/IA_Shoot.IA_Shoot"))
  ;[0 1 0.2865] Shoot
  (:`Triggered`
    (if (`/Game/Blueprints/Components/AC_Combat.Can Shoot Weapon` (`self.Combat Component`))
      (`/Game/Blueprints/Components/AC_Combat.Fire Equipped Weapon` (`self.Combat Component`) (`SceneComponent.GetForwardVector` (`self.Camera`)) (`self.Is Aiming`))
      (`|PlayMontage` (`self.Player Arms`) (`self.Get Fire Montage By Weapon`)))))

(event `EnhancedInput|/Game/Blueprints/Inputs/IA_Reload`
  (params (ActionValue :type Boolean) (ElapsedSeconds :type "Float (double-precision)") (TriggeredSeconds :type "Float (double-precision)") (InputAction :type "InputAction Object Reference" :default "/Game/Blueprints/Inputs/IA_Reload.IA_Reload"))
  (:`Started`
    (`|PlayMontage` (`self.Player Arms`) (`self.Get Reload Montage By Weapon`)
      (:`OnCompleted`
        (`/Game/Blueprints/Components/AC_Combat.Reload Equipped Weapon` (`self.Combat Component`))))))

(event `EnhancedInput|/Game/Blueprints/Inputs/IA_Weapon1`
  (params (ActionValue :type "Vector2D Structure") (ElapsedSeconds :type "Float (double-precision)") (TriggeredSeconds :type "Float (double-precision)") (InputAction :type "InputAction Object Reference" :default "/Game/Blueprints/Inputs/IA_Weapon1.IA_Weapon1"))
  ;[0 1 0.2865] Weapon 1
  (:`Started`
    (`/Game/Blueprints/Components/AC_Combat.Change Weapon` (`self.Combat Component`) "NewEnumerator0")))

(event `EnhancedInput|/Game/Blueprints/Inputs/IA_Weapon2`
  (params (ActionValue :type "Vector2D Structure") (ElapsedSeconds :type "Float (double-precision)") (TriggeredSeconds :type "Float (double-precision)") (InputAction :type "InputAction Object Reference" :default "/Game/Blueprints/Inputs/IA_Weapon2.IA_Weapon2"))
  ;[0 1 0.2865] Weapon 2
  (:`Started`
    (if (`/Game/Blueprints/Data/PDA_PlayerInventory.Has SMG` (`self.Player Inventory`))
      (`/Game/Blueprints/Components/AC_Combat.Change Weapon` (`self.Combat Component`) "NewEnumerator1"))))

(event `EnhancedInput|/Game/Blueprints/Inputs/IA_Weapon3`
  (params (ActionValue :type "Vector2D Structure") (ElapsedSeconds :type "Float (double-precision)") (TriggeredSeconds :type "Float (double-precision)") (InputAction :type "InputAction Object Reference" :default "/Game/Blueprints/Inputs/IA_Weapon3.IA_Weapon3"))
  ;[0 1 0.2865] Weapon 3
  (:`Started`
    (if (`/Game/Blueprints/Data/PDA_PlayerInventory.Has Rifle` (`self.Player Inventory`))
      (`/Game/Blueprints/Components/AC_Combat.Change Weapon` (`self.Combat Component`) "NewEnumerator2"))))

(event `EnhancedInput|/Game/Blueprints/Inputs/IA_Weapon4`
  (params (ActionValue :type "Vector2D Structure") (ElapsedSeconds :type "Float (double-precision)") (TriggeredSeconds :type "Float (double-precision)") (InputAction :type "InputAction Object Reference" :default "/Game/Blueprints/Inputs/IA_Weapon4.IA_Weapon4"))
  ;[0 1 0.2865] Weapon 4
  (:`Started`
    (if (`/Game/Blueprints/Data/PDA_PlayerInventory.Has Shotgun` (`self.Player Inventory`))
      (`/Game/Blueprints/Components/AC_Combat.Change Weapon` (`self.Combat Component`) "NewEnumerator3"))))

(fn `Get Fire Montage By Weapon`
  (returns (Montage :type "AnimMontage Object Reference"))
  (locals (Key :type String))
  (switch `/Game/Blueprints/Enums/E_PlayerWeapons` (`self.Current Weapon`)
    (:`NewEnumerator0`
      (set `local.Key` "Pistol"))
    (:`NewEnumerator1`
      (set `local.Key` "SMG"))
    (:`NewEnumerator2`
      (set `local.Key` "Rifle"))
    (:`NewEnumerator3`
      (set `local.Key` "Shotgun")))
  (if (`self.Is Aiming`)
    (return (`BlueprintMapLibrary.Map_Find` (`self.Fire Montages`) (`KismetStringLibrary.Concat_StrStr` (`local.Key`) "Aim")))
    (else
      (return (`BlueprintMapLibrary.Map_Find` (`self.Fire Montages`) (`local.Key`))))))

(fn `Get Reload Montage By Weapon`
  (returns (Montage :type "AnimMontage Object Reference"))
  (locals (Key :type String))
  (switch `/Game/Blueprints/Enums/E_PlayerWeapons` (`self.Current Weapon`)
    (:`NewEnumerator0`
      (set `local.Key` "Pistol"))
    (:`NewEnumerator1`
      (set `local.Key` "SMG"))
    (:`NewEnumerator2`
      (set `local.Key` "Rifle"))
    (:`NewEnumerator3`
      (set `local.Key` "Shotgun")))
  (return (`BlueprintMapLibrary.Map_Find` (`self.Reload Montages`) (`local.Key`))))

(fn `Is Aiming`
  (returns (ReturnValue :type Boolean))
  (return (`|EnumEquality` (`self.Player State`) "NewEnumerator1")))

(fn `Set New Player State`
  (params (`New Player State` :type "/Game/Blueprints/Enums/E_PlayerState Enum" :default "NewEnumerator0"))
  (bind _output_get (set `self.Player State` `New Player State`))
  (switch `/Game/Blueprints/Enums/E_PlayerState` _output_get
    (:`NewEnumerator0`
      (set `CharacterMovementComponent.MaxWalkSpeed` (`self.Walk Movement Speed`) (`self.CharacterMovement`)))
    (:`NewEnumerator1`
      (set `CharacterMovementComponent.MaxWalkSpeed` (`self.Aim Movement Speed`) (`self.CharacterMovement`)))
    (:`NewEnumerator3`
      (set `CharacterMovementComponent.MaxWalkSpeed` (`self.Run Movement Speed`) (`self.CharacterMovement`)))))

(fn `UserConstructionScript`)