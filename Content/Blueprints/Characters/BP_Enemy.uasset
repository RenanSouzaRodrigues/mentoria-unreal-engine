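; BP_Enemy is an enemy character that chases the player and takes damage until it dies.
; On BeginPlay it picks a random walk speed within its min/max range, then re-issues AI MoveTo toward player 0 on a short delay loop while alive.
; DealDamage lowers Health, always reporting no critical hit, and calls KillSelf at zero or below, which ragdolls the mesh and destroys the actor after a delay.
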(event `self.ReceiveBeginPlay`
  (set `CharacterMovementComponent.MaxWalkSpeed` (`KismetMathLibrary.RandomFloatInRange` (`self.Min Movement Speed`) (`self.Max Movement Speed`)) (`self.CharacterMovement`))
  (if (not (`self.Is Dead`)) :!label _label
    (`|AIMoveTo` self (0.0 0.0 0.0) (`GameplayStatics.GetPlayerCharacter` 0)
      (:`then`
        (`KismetSystemLibrary.Delay` 0.2)
        (goto _label)))))

(event `Kill Self`
  (set `self.Is Dead` true)
  (`PrimitiveComponent.SetCollisionEnabled` (`self.CapsuleComponent`) "NoCollision")
  (`PrimitiveComponent.SetCollisionEnabled` (`self.Mesh`) "QueryAndPhysics")
  (`PrimitiveComponent.SetSimulatePhysics` (`self.Mesh`) true)
  (`SkeletalMeshComponent.SetPhysicsBlendWeight` (`self.Mesh`) 1.0)
  (`KismetSystemLibrary.Delay` 5.0)
  (`self.K2_DestroyActor`))

(fn `Deal Damage`
  (params (Damage :type "Float (double-precision)"))
  (returns (`Damage Received` :type "Float (double-precision)") (`Critical Hit` :type Boolean))
  (set `self.Health` (- (`self.Health`) (`local.Damage`)))
  (if (<= (`self.Health`) 0.0)
    (`self.Kill Self`)
    (return (`local.Damage`) false)
    (else
      (return (`local.Damage`) false))))

(fn `UserConstructionScript`)