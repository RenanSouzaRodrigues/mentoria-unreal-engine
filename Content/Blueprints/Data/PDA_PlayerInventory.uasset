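; PDA_PlayerInventory is a player inventory data asset that holds money and ownership state for the SMG, rifle and shotgun.
; Getter functions report each weapon's state, and HasEnoughMoney tests whether the balance covers a given value.
; AddMoney and RemoveMoney adjust the balance directly, with RemoveMoney doing no affordability check or clamping of its own.
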(fn `Add Money`
  (params (Value :type Integer))
  (set `self.Money` (+ Value (`self.Money`))))

(fn `Has Enough Money`
  (params (Value :type Integer))
  (returns (ReturnValue :type Boolean))
  (return (>= (`self.Money`) (`local.Value`))))

(fn `Has Rifle`
  (returns (Rifle :type Boolean))
  (return (`self.Rifle`)))

(fn `Has Shotgun`
  (returns (Shotgun :type Boolean))
  (return (`self.Shotgun`)))

(fn `Has SMG`
  (returns (SMG :type Boolean))
  (return (`self.SMG`)))

(fn `Remove Money`
  (params (Value :type Integer))
  (set `self.Money` (- (`self.Money`) (`local.Value`))))