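; Weapon data asset (PDA) that holds a weapon's damage, spread and ammo values along with the logic that uses them.
; Damage is random within a range and doubles on criticals, while spread is random within separate aim and hip ranges.
; It tracks live clip and reserve counts itself, and Reload pools both to refill the clip.
; On a partial refill, the reserve becomes the old clip count instead of zero.
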(fn `Calculate Damage`
  (params (`Critical Hit` :type Boolean))
  (returns (ReturnValue :type "Float (double-precision)"))
  (locals (`Final Damage` :type "Float (double-precision)"))
  (set `local.Final Damage` (`KismetMathLibrary.RandomFloatInRange` (`self.Weapon Base Damage`) (`self.Weapon Max Damage`)))
  (if (`local.Critical Hit`)
    (return (* (`local.Final Damage`) 2.0))
    (else
      (return (`local.Final Damage`)))))

(fn `Calculate Spread`
  (params (`Is Aiming` :type Boolean))
  (returns (ReturnValue :type "Float (double-precision)"))
  (if `Is Aiming`
    (return (`KismetMathLibrary.RandomFloatInRange` (`self.Aim Weapon Min Spread`) (`self.Aim Weapon Max Spread`)))
    (else
      (return (`KismetMathLibrary.RandomFloatInRange` (`self.Weapon Min Spread`) (`self.Weapon Max Spred`))))))

(fn `Has Ammo`
  (returns (ReturnValue :type Boolean))
  (return (> (`self.Current Clip Amount`) 0)))

(fn `Reload`
  (locals (`Final Ammo Count` :type Integer))
  (if (> (`self.Current Ammo Count`) 0)
    ;[0.5843 1 0.8943] Pegamos o quanto sobrou de munição na nossa arma e somamos com a quantidade que temos de reserva. Salvando em uma variavel temporaria
    (set `local.Final Ammo Count` (+ (`self.Current Clip Amount`) (`self.Current Ammo Count`)))
    (if (> (`self.Clip Size`) (`local.Final Ammo Count`))
      (set `self.Current Clip Amount` (`local.Final Ammo Count`))
      (set `self.Current Ammo Count` (- (`local.Final Ammo Count`) (`self.Current Ammo Count`)))
      (else
        (set `self.Current Clip Amount` (`self.Clip Size`))
        (set `self.Current Ammo Count` (- (`local.Final Ammo Count`) (`self.Clip Size`)))))))

(fn `Subtract Ammo From Clip`
  (`/Engine/EditorBlueprintResources/StandardMacros.DecrementInt` (`self.Current Clip Amount`)))